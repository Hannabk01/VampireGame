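; NPC dialogue component that shows a dialogue bubble when triggered while the player overlaps the owning actor.
; On BeginPlay it creates a hidden widget component with the dialogue text widget and binds the owner's overlap events.
; Triggering dialogue reveals the bubble, passes DialogueDT to player and widget, and, if an interact pop-up component exists, notifies it and teleports the player near PlayerLocation.
; Ending dialogue notifies that pop-up component.
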(event `self.ReceiveBeginPlay`
  (bind _returnvalue (`self.GetOwner`))
  (`|ExecutionSequence`
    (:`then_0`
      ;[0.05781 0.5333 0.5776 0.502] EVENT BEGIN PLAY: Create a widget component, set it's details, and then set the widget as the NPC dialogue widget
      (bind _returnvalue_2 (`|AddComponentByClass` (`self.GetOwner`) "/Script/UMG.WidgetComponent" false (`self.DialogueWidget_Location`)))
      (bind _output_get (set `self.WidgetComponentREF` _returnvalue_2))
      (`WidgetComponent.SetDrawSize` _output_get (500.0 500.0))
      (`WidgetComponent.SetWidgetSpace` _returnvalue_2 (`self.DialogueWidget_ScreenSpace`))
      (`PrimitiveComponent.SetCollisionEnabled` _returnvalue_2 "NoCollision")
      (`PrimitiveComponent.SetMaterial` _returnvalue_2 0 "/Game/Materials/M_DialogueUI.M_DialogueUI")
      (`SceneComponent.SetVisibility` _returnvalue_2 false false)
      (bind _returnvalue_3 (`|CreateWidget` "/Game/Systems/Dialogue/WBP_NPC_Dialogue_TEXT.WBP_NPC_Dialogue_TEXT_C"))
      (bind _output_get_2 (set `self.DialogueWidgetREFs` _returnvalue_3))
      (`WidgetComponent.SetWidget` (`self.WidgetComponentREF`) _output_get_2))
    (:`then_1`
      ;[0.05781 0.5333 0.5776 0.502] Create REF to Interact Component
      (set `self.InteractComponentREF` (`Actor.GetComponentByClass` (`self.GetOwner`) "/Game/Systems/Interact/AC_InteractPopUp.AC_InteractPopUp_C"))
      (bind _asbp_third_person_character (cast `/Game/Player/BP_ThirdPersonCharacter` (`GameplayStatics.GetPlayerCharacter` 0)))
      (set `self.PlayerREF` _asbp_third_person_character))
    (:`then_2`
      ;[0.3005 0.5583 0.1746 0.502] Determine wether player is overlapping owning actor or not based on On Actor Begin/End Overlap events. Trigger boolean accordingly.
      (add `Actor.OnActorBeginOverlap` _returnvalue (delegate `OnActorBeginOverlap_Event`))
      (add `Actor.OnActorEndOverlap` _returnvalue (delegate `OnActorEndOverlap_Event`)))))

(event `OnActorBeginOverlap_Event`
  (params (OverlappedActor :type "Actor Object Reference") (OtherActor :type "Actor Object Reference"))
  ;[0.3005 0.5583 0.1746 0.502] Determine wether player is overlapping owning actor or not based on On Actor Begin/End Overlap events. Trigger boolean accordingly.
  (if (== OtherActor (`GameplayStatics.GetPlayerCharacter` 0))
    (set `self.PlayerOverlapping?` true)))

(event `OnActorEndOverlap_Event`
  (params (OverlappedActor :type "Actor Object Reference") (OtherActor :type "Actor Object Reference"))
  ;[0.3005 0.5583 0.1746 0.502] Determine wether player is overlapping owning actor or not based on On Actor Begin/End Overlap events. Trigger boolean accordingly.
  (if (== OtherActor (`GameplayStatics.GetPlayerCharacter` 0))
    (set `self.PlayerOverlapping?` false)))

(event `Dialogue Triggered`
  (bind _dialogue_dt (`self.Dialogue_DT`))
  (bind _interactcomponentref (`self.InteractComponentREF`))
  ;[0.9216 0.7605 0.15 0.502] CONVERSATION INTERACT: When player interacts with NPC (presses 'E' and is close enough) Open or close the dialogue bubble
  (`self.PlayerOverlapping?`
    (:`then`
      (`/Game/Player/BP_ThirdPersonCharacter.InDialogue?` (`self.PlayerREF`)
        (:`then`)
        (:`else`
          (`SceneComponent.SetVisibility` (`self.WidgetComponentREF`) true false)
          (message `/Game/Systems/Dialogue/BPI_DialogueNEW.TriggerDialogue` (`GameplayStatics.GetPlayerCharacter` 0) _dialogue_dt)
          (message `/Game/Systems/Dialogue/BPI_DialogueNEW.TriggerDialogue` (`self.DialogueWidgetREFs`) _dialogue_dt)
          ;; Hides Interact Widget
          (`/Engine/EditorBlueprintResources/StandardMacros.IsValid` _interactcomponentref
            (:`Is Valid`
              (`/Game/Systems/Interact/AC_InteractPopUp.PlayerEntersDialogue` _interactcomponentref)
              (`self.SetPlayerLocation`))))))
    (:`else`)))

(event `DialogueEnded`
  (bind _interactcomponentref (`self.InteractComponentREF`))
  ;[0.9216 0.7605 0.15 0.502] CONVERSATION ENDS: Make interact widget visible again
  (`self.PlayerOverlapping?`
    (:`then`
      (`/Engine/EditorBlueprintResources/StandardMacros.IsValid` _interactcomponentref
        (:`Is Valid`
          (`/Game/Systems/Interact/AC_InteractPopUp.PlayerExitsDialogue` _interactcomponentref))))
    (:`else`)))

(event `SetPlayerLocation`
  (bind _returnvalue (`GameplayStatics.GetPlayerCharacter` 0))
  (bind (_playerlocation_location _playerlocation_rotation) (`KismetMathLibrary.BreakTransform` (`self.PlayerLocation`)))
  ;[0.8854 0.3837 0 0.5] Transition player to location/rotation of "Player Location" variable
  (`Actor.K2_SetActorLocationAndRotation` _returnvalue (`KismetMathLibrary.VInterpTo` (`KismetMathLibrary.TransformLocation` (`Actor.GetTransform` (`self.GetOwner`)) _playerlocation_location) (`Actor.K2_GetActorLocation` _returnvalue) (`GameplayStatics.GetWorldDeltaSeconds`) 1.0) _playerlocation_rotation false true))

(fn `Interact`
  (returns (`Sucess?` :type Boolean))
  (return false))