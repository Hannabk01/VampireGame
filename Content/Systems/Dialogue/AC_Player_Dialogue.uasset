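; Player actor component that runs dialogue, creating a widget component on its owner to show the player dialogue UI.
; Triggering dialogue disables movement, moves the spring-arm camera with lag and clamps view angles, and ending it restores both.
; Input skips typewriter text or advances lines through BPI_Dialogue widgets, and cycles or selects options.
; Dialogue state and typewriter flags live in GI_VampGameInstance.
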(event `self.ReceiveBeginPlay`
  (bind _returnvalue (`Actor.GetComponentByClass` (`self.GetOwner`) "/Script/Engine.MovementComponent"))
  (bind _returnvalue_2 (`Actor.GetComponentByClass` (`self.GetOwner`) "/Script/Engine.SpringArmComponent"))
  ;[0.6105 0.05951 0.05951 0.502] BEGIN PLAY
  (`|ExecutionSequence`
    (:`then_0`
      ;[0.05781 0.5333 0.5776 0.502] EVENT BEGIN PLAY: Create a widget component, set it's details, and then set the widget as the Player dialogue widget
      (bind _returnvalue_3 (`|AddComponentByClass` (`self.GetOwner`) "/Script/UMG.WidgetComponent" false (`self.DialogueWidget_Location`)))
      (bind _output_get (set `self.WidgetComponentREF` _returnvalue_3))
      (`WidgetComponent.SetDrawSize` _output_get (500.0 500.0))
      (`WidgetComponent.SetWidgetSpace` _returnvalue_3 (`self.DialogueWidget_ScreenSpace`))
      (`PrimitiveComponent.SetCollisionEnabled` _returnvalue_3 "NoCollision")
      (`PrimitiveComponent.SetMaterial` _returnvalue_3 0 "/Game/Materials/M_DialogueUI.M_DialogueUI")
      (`SceneComponent.SetVisibility` _returnvalue_3 false false)
      (bind _returnvalue_4 (`|CreateWidget` "/Game/Systems/Dialogue/WBP_Player_Dialogue.WBP_Player_Dialogue_C"))
      (bind _output_get_2 (set `self.DialogueWidget_REF` _returnvalue_4))
      (`WidgetComponent.SetWidget` (`self.WidgetComponentREF`) _output_get_2))
    (:`then_1`
      ;[0.05781 0.5333 0.5776 0.502] REFS
      (bind _asgi_vamp_game_instance (cast `/Game/Player/GI_VampGameInstance` (`GameplayStatics.GetGameInstance`)))
      (set `self.GameInstance_REF` _asgi_vamp_game_instance)
      (`/Engine/EditorBlueprintResources/StandardMacros.IsValid` _returnvalue_2
        (:`Is Valid`
          (set `self.CameraBoom` _returnvalue_2))
        (:`Is Not Valid`
          _))
      (`/Engine/EditorBlueprintResources/StandardMacros.IsValid` _returnvalue
        (:`Is Valid`
          (set `self.CharacterMovement` _returnvalue))))))

(event `/Game/Systems/Dialogue/BPI_Dialogue.TriggerDialogue`
  (params (`Dialogue DataTable` :type "DataTable Object Reference"))
  ;[0.9216 0.7605 0.15 0.502] DIALOGUE Triggered: Limit Camera Movement
  (`/Game/Player/GI_VampGameInstance.InDialogue` (`self.GameInstance_REF`)
    (:`then`)
    (:`else`
      (`SceneComponent.SetVisibility` (`self.WidgetComponentREF`) true false)
      (message `/Game/Systems/Dialogue/BPI_Dialogue.TriggerDialogue` (`self.DialogueWidget_REF`) `Dialogue DataTable`)
      (`CharacterMovementComponent.DisableMovement` (`self.CharacterMovement`))
      (`self.DialogueCamera`)
      (set `/Game/Player/GI_VampGameInstance.InDialogue` true (`self.GameInstance_REF`))
      (`KismetSystemLibrary.Delay` 1.0)
      (`self.CameraMovement_LIMITED`)
      (set `SpringArmComponent.bUsePawnControlRotation` true (`self.CameraBoom`)))))

(event `/Game/Systems/Dialogue/BPI_Dialogue.TriggerOptionsDialogue`
  (params (OptionsDialogue_DataTable :type "DataTable Object Reference"))
  ;[0.9216 0.7605 0.15 0.502] DIALOGUE OPTIONS Triggered
  (message `/Game/Systems/Dialogue/BPI_Dialogue.TriggerOptionsDialogue` (`self.DialogueWidget_REF`) OptionsDialogue_DataTable))

(event `/Game/Systems/Dialogue/BPI_Dialogue.EndDialogue`
  (bind _gameinstance_ref (`self.GameInstance_REF`))
  ;[0.9216 0.7605 0.15 0.502] DIALOGUE Ended: Set camera t be free
  (`CharacterMovementComponent.SetMovementMode` (`self.CharacterMovement`) "MOVE_Walking" 0)
  (`self.CameraMovement_FREE`)
  (`SceneComponent.SetVisibility` (`self.WidgetComponentREF`) false false)
  (set `/Game/Player/GI_VampGameInstance.InDialogue` false _gameinstance_ref)
  (set `/Game/Player/GI_VampGameInstance.SoloDialogue?` false _gameinstance_ref))

(event `/Game/Systems/Dialogue/BPI_Dialogue.Force_Continue`
  (bind _gameinstance_ref (`self.GameInstance_REF`))
  ;[0.9216 0.7605 0.15 0.502] DIALOGUE: Continue Dialogue
  (bind _result (`/Engine/EditorBlueprintResources/StandardMacros.IncrementInt` (`/Game/Player/GI_VampGameInstance.Dialogue_Index` _gameinstance_ref) :!label _label)
    (:`  `
      (set `/Game/Player/GI_VampGameInstance.Dialogue_Index` _result _gameinstance_ref)
      (bind _foundwidgets (`WidgetBlueprintLibrary.GetAllWidgetsWithInterface` "/Game/Systems/Dialogue/BPI_Dialogue.BPI_Dialogue_C"))
      (for _array_element _foundwidgets
        (message `/Game/Systems/Dialogue/BPI_Dialogue.ContinueDialogue` _array_element)))))

(event `EnhancedInput|/Game/Player/Input/Actions/IA_ContinueDialogue`
  (params (ActionValue :type Boolean) (ElapsedSeconds :type "Float (double-precision)") (TriggeredSeconds :type "Float (double-precision)") (InputAction :type "InputAction Object Reference" :default "/Game/Player/Input/Actions/IA_ContinueDialogue.IA_ContinueDialogue"))
  (bind _gameinstance_ref (`self.GameInstance_REF`))
  (bind _gameinstance_ref_2 (`self.GameInstance_REF`))
  (bind _player_typewriterfinished (`/Game/Player/GI_VampGameInstance.Player_TypewriterFinished` _gameinstance_ref_2))
  ;[0.9216 0.7605 0.15 0.502] DIALOGUE: Continue Dialogue
  (:`Completed`
    (`/Game/Player/GI_VampGameInstance.InDialogue` _gameinstance_ref
      (:`then`
        (`/Game/Player/GI_VampGameInstance.Options?` _gameinstance_ref
          (:`then`)
          (:`else`
            (`/Game/Player/GI_VampGameInstance.SoloDialogue?` _gameinstance_ref
              (:`then`
                (if _player_typewriterfinished
                  (goto _label)
                  (else
                    _)))
              (:`else`
                (if (and _player_typewriterfinished (`/Game/Player/GI_VampGameInstance.NPC_TypewriterFinished` _gameinstance_ref_2))
                  (goto _label)
                  (else
                    _))))
            (bind _foundwidgets (`WidgetBlueprintLibrary.GetAllWidgetsWithInterface` "/Game/Systems/Dialogue/BPI_Dialogue.BPI_Dialogue_C"))
            (for _array_element _foundwidgets
              (message `/Game/Systems/Dialogue/BPI_Dialogue.TypewritersFinished` _array_element)))))
      (:`else`))))

(event `EnhancedInput|/Game/Player/Input/Actions/IA_Down`
  (params (ActionValue :type Boolean) (ElapsedSeconds :type "Float (double-precision)") (TriggeredSeconds :type "Float (double-precision)") (InputAction :type "InputAction Object Reference" :default "/Game/Player/Input/Actions/IA_Down.IA_Down"))
  (bind _gameinstance_ref (`self.GameInstance_REF`))
  ;[0.9216 0.7605 0.15 0.502] Turn Mouse Wheel (Up or down) to cycle through the different options
  (:`Started`
    (`/Game/Player/GI_VampGameInstance.InDialogue` _gameinstance_ref
      (:`then`
        (`/Game/Player/GI_VampGameInstance.Options?` _gameinstance_ref
          (:`then`
            (`/Game/Systems/Dialogue/BPI_Dialogue.Select Next` (`self.DialogueWidget_REF`)))
          (:`else`)))
      (:`else`))))

(event `EnhancedInput|/Game/Player/Input/Actions/IA_Up`
  (params (ActionValue :type Boolean) (ElapsedSeconds :type "Float (double-precision)") (TriggeredSeconds :type "Float (double-precision)") (InputAction :type "InputAction Object Reference" :default "/Game/Player/Input/Actions/IA_Up.IA_Up"))
  (bind _gameinstance_ref (`self.GameInstance_REF`))
  ;[0.9216 0.7605 0.15 0.502] Turn Mouse Wheel (Up or down) to cycle through the different options
  (:`Started`
    (`/Game/Player/GI_VampGameInstance.InDialogue` _gameinstance_ref
      (:`then`
        (`/Game/Player/GI_VampGameInstance.Options?` _gameinstance_ref
          (:`then`
            (`/Game/Systems/Dialogue/BPI_Dialogue.Select Previous` (`self.DialogueWidget_REF`)))
          (:`else`)))
      (:`else`))))

(event `EnhancedInput|/Game/Player/Input/Actions/IA_SelectDialogue`
  (params (ActionValue :type Boolean) (ElapsedSeconds :type "Float (double-precision)") (TriggeredSeconds :type "Float (double-precision)") (InputAction :type "InputAction Object Reference" :default "/Game/Player/Input/Actions/IA_SelectDialogue.IA_SelectDialogue"))
  (bind _gameinstance_ref (`self.GameInstance_REF`))
  ;[0.9216 0.7605 0.15 0.502] When LMB or Enter is pressed: Check to see if the dialogue widget is visible, if it is trigger select current event to select the option currently hoevered on
  (:`Started`
    (`/Game/Player/GI_VampGameInstance.InDialogue` _gameinstance_ref
      (:`then`
        (`/Game/Player/GI_VampGameInstance.Options?` _gameinstance_ref
          (:`then`
            (`/Game/Systems/Dialogue/BPI_Dialogue.Select Current` (`self.DialogueWidget_REF`)))
          (:`else`)))
      (:`else`))))

(fn `CameraMovement_FREE`
  (bind _returnvalue (`GameplayStatics.GetPlayerCameraManager` 0))
  (bind _cameraboom (`self.CameraBoom`))
  ; Camera lag is disabled
  (set `SpringArmComponent.bUsePawnControlRotation` true (`self.CameraBoom`))
  (set `SpringArmComponent.bEnableCameraLag` false _cameraboom)
  (set `SpringArmComponent.bEnableCameraRotationLag` false _cameraboom)
  ; Limit the cameras movement based on the MAX and MIN
  (set `self.MAX` 359.99)
  (set `self.MIN` -359.99)
  (set `PlayerCameraManager.ViewPitchMax` (`self.MAX`) _returnvalue)
  (set `PlayerCameraManager.ViewPitchMin` (`self.MIN`) _returnvalue)
  (set `PlayerCameraManager.ViewRollMax` (`self.MAX`) _returnvalue)
  (set `PlayerCameraManager.ViewRollMin` (`self.MIN`) _returnvalue)
  (set `PlayerCameraManager.ViewYawMax` (`self.MAX`) _returnvalue)
  (set `PlayerCameraManager.ViewYawMin` (`self.MIN`) _returnvalue))

(fn `CameraMovement_LIMITED`
  (bind _returnvalue (`GameplayStatics.GetPlayerCameraManager` 0))
  (bind (_returnvalue_roll _returnvalue_pitch _returnvalue_yaw) (`KismetMathLibrary.BreakRotator` (`SpringArmComponent.GetTargetRotation` (`self.CameraBoom`))))
  ; Limit the cameras movement based on the MAX and MIN
  (set `self.MAX` 10.0)
  (set `self.MIN` -10.0)
  (set `PlayerCameraManager.ViewPitchMax` (+ _returnvalue_pitch 0.0) _returnvalue)
  (set `PlayerCameraManager.ViewPitchMin` (+ _returnvalue_pitch -20.0) _returnvalue)
  (set `PlayerCameraManager.ViewRollMax` (+ _returnvalue_roll (`self.MAX`)) _returnvalue)
  (set `PlayerCameraManager.ViewRollMin` (+ _returnvalue_roll (`self.MIN`)) _returnvalue)
  (set `PlayerCameraManager.ViewYawMax` (+ _returnvalue_yaw (`self.MAX`)) _returnvalue)
  (set `PlayerCameraManager.ViewYawMin` (+ _returnvalue_yaw (`self.MIN`)) _returnvalue))

(fn `DialogueCamera`
  (bind _cameraboom (`self.CameraBoom`))
  ; Set camera to move to desired realtive location, and enable lag
  (set `SpringArmComponent.bUsePawnControlRotation` false _cameraboom)
  (`SceneComponent.K2_SetRelativeRotation` _cameraboom (struct :`Yaw` -30.0) false false)
  (set `SpringArmComponent.bEnableCameraLag` true _cameraboom)
  (set `SpringArmComponent.bEnableCameraRotationLag` true _cameraboom)
  (set `SpringArmComponent.CameraRotationLagSpeed` 1.5 _cameraboom)
  (set `SpringArmComponent.CameraLagSpeed` 1.0 _cameraboom))