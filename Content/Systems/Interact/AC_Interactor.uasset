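; AC_Interactor is an interaction component that lets its owner trigger nearby actors when the IA_Interact input fires.
; Each press first calls its own Interact function, which just returns false and is commented as resetting the success flag.
; It then sphere-overlaps Pawn, WorldStatic and WorldDynamic objects around the owner.
; It sends each overlapped actor an Interact message, stopping at the first that returns true.
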(event `EnhancedInput|/Game/Player/Input/Actions/IA_Interact`
  (params (ActionValue :type Boolean) (ElapsedSeconds :type "Float (double-precision)") (TriggeredSeconds :type "Float (double-precision)") (InputAction :type "InputAction Object Reference" :default "/Game/Player/Input/Actions/IA_Interact.IA_Interact"))
  ;[0.3005 0.5583 0.1746 0.502] INTERACT: Press 'E' to resset sucess bool, and then check for any Pawns, WordStatic, or WorldDynamic actors within player radius. If found any, trigger their Interact event.
  (:`Triggered`
    (`|ExecutionSequence`
      (:`then_0`
        (`/Game/Systems/Interact/BPI_Interact.Interact`))
      (:`then_1`
        (bind _outactors (`KismetSystemLibrary.SphereOverlapActors` (`Actor.K2_GetActorLocation` (`self.GetOwner`)) 90.0 (`|MakeArray` "ObjectTypeQuery3" "ObjectTypeQuery1" "ObjectTypeQuery2" :!type "EObjectTypeQuery Enum")))
        (for _array_element _outactors
          (bind _sucess_ (message `/Game/Systems/Interact/BPI_Interact.Interact` _array_element))
          (if _sucess_
            (break)))))))

(fn `Interact`
  (returns (`Sucess?` :type Boolean))
  (return false))