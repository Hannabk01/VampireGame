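; Actor component that shows an interaction prompt widget on its owning actor when the player overlaps it.
; On BeginPlay it adds a configurable, hidden WidgetComponent holding WBP_Interact, with a dialogue or object icon chosen by InteractionType.
; It binds the owner's overlap events to fade the prompt in and out for the player character.
; Dialogue enter and exit events hide it and restore it if the player still overlaps.
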(event `self.ReceiveBeginPlay`
  (bind _returnvalue (`self.GetOwner`))
  (bind _interact_image (`/Game/Widgets/WBP_Interact.Interact_Image` (`self.InteractWidgetREF`)))
  (`|ExecutionSequence`
    (:`then_0`
      ;[0.3005 0.5583 0.1746 0.502] Add a Widget Component to actor (used to add place for widget to be displayed), set it's information (can be changed in actor), and set image type for widget to display based on ENUM choice.
      (bind _returnvalue_2 (`|AddComponentByClass` (`self.GetOwner`) "/Script/UMG.WidgetComponent" false (`self.Widget_Transform`)))
      (bind _output_get (set `self.WidgetComponentREF` _returnvalue_2))
      (`WidgetComponent.SetDrawSize` _output_get (`self.Widget_DrawSize`))
      (`WidgetComponent.SetWidgetSpace` _returnvalue_2 (`self.Widget_Space`))
      (`PrimitiveComponent.SetCollisionEnabled` _returnvalue_2 "NoCollision")
      (`PrimitiveComponent.SetMaterial` _returnvalue_2 0 "/Engine/EngineMaterials/Widget3DPassThrough_Translucent.Widget3DPassThrough_Translucent")
      (`SceneComponent.SetVisibility` _returnvalue_2 false false)
      (bind _returnvalue_3 (`|CreateWidget` "/Game/Widgets/WBP_Interact.WBP_Interact_C"))
      (bind _output_get_2 (set `self.InteractWidgetREF` _returnvalue_3))
      (`WidgetComponent.SetWidget` (`self.WidgetComponentREF`) _output_get_2)
      (switch `/Game/Systems/Interact/Enum_InteractWidgetDisplay` (`self.InteractionType`)
        (:`NewEnumerator0`
          (`Image.SetBrush` _interact_image (`self.Widget_DialogueImage`)))
        (:`NewEnumerator1`
          (`Image.SetBrush` _interact_image (`self.Widget_ObjectImage`)))))
    (:`then_1`
      ;[0.5583 0.7157 0.2462 0.502] When owning actor has actor begin and end overlap triggered, bind to event in this blueprint.
      (add `Actor.OnActorBeginOverlap` _returnvalue (delegate `OnActorBeginOverlap_Event`))
      (add `Actor.OnActorEndOverlap` _returnvalue (delegate `OnActorEndOverlap_Event`)))))

(event `OnActorBeginOverlap_Event`
  (params (OverlappedActor :type "Actor Object Reference") (OtherActor :type "Actor Object Reference"))
  (bind _interactwidgetref (`self.InteractWidgetREF`))
  ;[0.5583 0.7157 0.2462 0.502] When PlayerBeginOverlap event is called from actor blueprint, trigger the widget to appear
  (if (== OtherActor (`GameplayStatics.GetPlayerCharacter` 0))
    (set `self.PlayerOverlaping?` true)
    (`SceneComponent.SetVisibility` (`self.WidgetComponentREF`) true false)
    (`UserWidget.PlayAnimation` _interactwidgetref (`/Game/Widgets/WBP_Interact.FadeIn` _interactwidgetref) 0.0 1 "Forward" 1.0 false)))

(event `OnActorEndOverlap_Event`
  (params (OverlappedActor :type "Actor Object Reference") (OtherActor :type "Actor Object Reference"))
  (bind _interactwidgetref (`self.InteractWidgetREF`))
  ;[0.5588 0.7188 0.247 0.502] When PlayerEndOverlap event is called from actor blueprint, trigger the widget to disappear
  (if (== OtherActor (`GameplayStatics.GetPlayerCharacter` 0))
    (set `self.PlayerOverlaping?` false)
    (`UserWidget.PlayAnimation` _interactwidgetref (`/Game/Widgets/WBP_Interact.FadeOut` _interactwidgetref) 0.0 1 "Forward" 1.0 false)
    (`KismetSystemLibrary.Delay` 0.15)
    (`SceneComponent.SetVisibility` (`self.WidgetComponentREF`) false false)))

(event `PlayerEntersDialogue`
  (bind _interactwidgetref (`self.InteractWidgetREF`))
  ; When Player has entered dialogue, fade out the interact widget
  (`UserWidget.PlayAnimation` _interactwidgetref (`/Game/Widgets/WBP_Interact.FadeOut` _interactwidgetref) 0.0 1 "Forward" 1.0 false)
  (`KismetSystemLibrary.Delay` 0.15)
  (`SceneComponent.SetVisibility` (`self.WidgetComponentREF`) false false))

(event `PlayeExitsDialogue`
  (bind _interactwidgetref (`self.InteractWidgetREF`))
  ; When Player exits dialogue, fade in the interact widget
  (if (`self.PlayerOverlaping?`)
    (`KismetSystemLibrary.Delay` 0.2)
    (`SceneComponent.SetVisibility` (`self.WidgetComponentREF`) true false)
    (`UserWidget.PlayAnimation` _interactwidgetref (`/Game/Widgets/WBP_Interact.FadeIn` _interactwidgetref) 0.0 1 "Forward" 1.0 false)))