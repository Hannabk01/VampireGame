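; Player controller that lets the player switch between Vampire and Bat characters.
; BeginPlay adds the abilities input mapping, finds both tagged characters and creates the bat stamina HUD.
; IA_Transform hides one pawn and possesses the other, carrying over transform, control rotation and velocity; returning to Vampire requires non-zero BatStamina.
; ForceTransformtoVampire actually calls TransformToBat, and the Transform function is empty with disconnected logic.
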(event `CreateHUD`
  ;[0.05781 0.5333 0.5776 0.502] Create HUD and Set Input Mode to GAME
  (bind _returnvalue (`|CreateWidget` "/Game/Systems/BatStamina/WBP_BatStamina.WBP_BatStamina_C"))
  (bind _output_get (set `self.BatStamina_REF` _returnvalue))
  (`UserWidget.AddToViewport` _output_get 0)
  (`WidgetBlueprintLibrary.SetInputMode_GameOnly` (`GameplayStatics.GetPlayerController` 0)))

(event `self.ReceiveBeginPlay`
  ;[0.5938 0.1098 0.09444 0.4087] BEGIN PLAY
  (`self.Set Mapping Context`)
  (`self.Set Player Characters`)
  (`self.CreateHUD`)
  (`self.Set Game Instance`)
  (`self.Set Player REF`))

(event `Set Mapping Context`
  ;[0.05781 0.5333 0.5776 0.502] Set the Abilities mapping context (makes sure all player states can use it smoothly)
  (`EnhancedInputSubsystemInterface.AddMappingContext` (pcsubsystem `EnhancedInputLocalPlayerSubsystem` self) "/Game/Player/Input/IMC_Abilities.IMC_Abilities" 0 (struct)))

(event `Set Player Characters`
  ;[0.05781 0.5333 0.5776 0.502] Set Player Characters (creates references used to switch between characters)
  (bind _outactors (`GameplayStatics.GetAllActorsOfClassWithTag` "/Script/Engine.Character" "PlayerCharacter"))
  (bind _output_get (set `self.PlayerCharacters` _outactors))
  (set `self.Vampire` (`|GetArrayItem` _output_get))
  (set `self.Bat` (`|GetArrayItem` _output_get 1)))

(event `Set Game Instance`
  ;[0.05781 0.5333 0.5776 0.502] Set Game Instance REF
  (bind _asgi_vamp_game_instance (cast `/Game/Player/GI_VampGameInstance` (`GameplayStatics.GetGameInstance`)))
  (set `self.GameInstance_REF` _asgi_vamp_game_instance))

(event `Set Player REF`
  (bind _asbp_third_person_character (cast `/Game/Player/BP_ThirdPersonCharacter` (`GameplayStatics.GetPlayerCharacter` 0)))
  (set `self.VampirePlayer_REF` _asbp_third_person_character))

(event `EnhancedInput|/Game/Player/Input/Actions/IA_Transform`
  (params (ActionValue :type Boolean) (ElapsedSeconds :type "Float (double-precision)") (TriggeredSeconds :type "Float (double-precision)") (InputAction :type "InputAction Object Reference" :default "/Game/Player/Input/Actions/IA_Transform.IA_Transform"))
  ;[0.849 0.2616 0.09285] When Tranform started (Alt clicked), check to see if vampire character is currently possesed, and trigger correct event.
  (:`Started`
    (if (== (`self.Vampire`) (`self.K2_GetPawn`))
      (`/Game/Systems/Transform/BPI_TransformPlayer.TransformToBat` :!label _label)
      (elif (not (== (`/Game/Player/GI_VampGameInstance.Bat_Stamina` (`self.GameInstance_REF`)) 0.0))
        (`/Game/Systems/Transform/BPI_TransformPlayer.TransformToVampire`)))))

(event `/Game/Systems/Transform/BPI_TransformPlayer.ForceTransformToVampire`
  ;[0.849 0.2616 0.09285] When Tranform started (Alt clicked), check to see if vampire character is currently possesed, and trigger correct event.
  (goto _label))

(event `/Game/Systems/Transform/BPI_TransformPlayer.TransformToBat`
  (bind _vampire (`self.Vampire`))
  (bind _bat (`self.Bat`))
  (bind _bat_2 (`self.Bat`))
  (bind _playercameramanager (`self.PlayerCameraManager`))
  ;[0.849 0.2616 0.09285] Transform to Bat: hide the vampire actor, posses bat actor and transform to bat current position, and unhide bat actor
  (`|ExecutionSequence`
    (:`then_0`
      (`self.SetActorHiddenInGame` _vampire true)
      (`self.SetActorEnableCollision` _vampire false)
      (set `self.PlayerTransform` (`self.GetTransform` _vampire))
      (set `self.PlayerControlRotation` (`Pawn.GetControlRotation` _vampire))
      (set `self.PlayerCameraLocation` (`PlayerCameraManager.GetCameraLocation` _playercameramanager))
      (set `self.PlayerCameraRotation` (`PlayerCameraManager.GetCameraRotation` _playercameramanager))
      (set `self.PlayerVelocity` (`MovementComponent.Velocity` (`Character.CharacterMovement` (`self.Vampire`)))))
    (:`then_1`
      (set `self.PlayerCameraLocation` (`self.PlayerCameraLocation`))
      (set `self.PlayerCameraRotation` (`self.PlayerCameraRotation`))
      (`self.Possess` _bat)
      (`self.SetActorHiddenInGame` _bat false)
      (`self.SetActorEnableCollision` _bat true)
      (`self.K2_SetActorTransform` _bat (`self.PlayerTransform`) false true)
      (`self.SetControlRotation` (`self.PlayerControlRotation`))
      (set `MovementComponent.Velocity` (`self.PlayerVelocity`) (`Character.CharacterMovement` _bat_2))
      (message `/Game/Systems/Transform/BPI_TransformPlayer.ActivateTransformPoof` _bat_2))))

(event `/Game/Systems/Transform/BPI_TransformPlayer.TransformToVampire`
  (bind _vampire (`self.Vampire`))
  (bind _bat (`self.Bat`))
  (bind _vampire_2 (`self.Vampire`))
  (bind _playercameramanager (`self.PlayerCameraManager`))
  ;[0.849 0.2616 0.09285] Transform to Vampire: hide the bat actor, posses vampire actor and transform to bat current position, and unhide vampire actor
  (`|ExecutionSequence`
    (:`then_0`
      (`self.SetActorHiddenInGame` _bat true)
      (`self.SetActorEnableCollision` _bat false)
      (set `self.PlayerTransform` (`self.GetTransform` _bat))
      (set `self.PlayerControlRotation` (`Pawn.GetControlRotation` _bat))
      (set `self.PlayerCameraLocation` (`PlayerCameraManager.GetCameraLocation` _playercameramanager))
      (set `self.PlayerCameraRotation` (`PlayerCameraManager.GetCameraRotation` _playercameramanager))
      (set `self.PlayerVelocity` (`MovementComponent.Velocity` (`Character.CharacterMovement` (`self.Bat`)))))
    (:`then_1`
      (set `self.PlayerCameraLocation` (`self.PlayerCameraLocation`))
      (set `self.PlayerCameraRotation` (`self.PlayerCameraRotation`))
      (`self.Possess` _vampire)
      (`self.SetActorHiddenInGame` _vampire false)
      (`self.SetActorEnableCollision` _vampire true)
      (`self.K2_SetActorTransform` _vampire (`self.PlayerTransform`) false true)
      (`self.SetControlRotation` (`self.PlayerControlRotation`))
      (set `MovementComponent.Velocity` (`self.PlayerVelocity`) (`Character.CharacterMovement` _vampire_2))
      (message `/Game/Systems/Transform/BPI_TransformPlayer.ActivateTransformPoof` _vampire_2))))

(fn `Transform`
  (params (Vampire :type "Character Object Reference") (Bat :type "Character Object Reference"))
  ; Check to see if player is currently vampire or not (if adding more modes later add more branching checks)
)

(fn `UserConstructionScript`)