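; Player transform component that toggles between human and bat forms on IA_Transform, with ForceHumanTransform to force the human branch.
; Bat form swaps the skeletal mesh; human form re-shows and activates it without restoring the asset.
; SetBatGravity runs once per switch to bat, setting gravity and air control and, if falling, clamping vertical velocity tighter when moving for gliding.
; Each switch sets Falling mode and fires PoofActivated.
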(event `self.ReceiveBeginPlay`
  (bind _returnvalue (`GameplayStatics.GetPlayerCharacter` 0))
  ; Create Charater Movement and Mesh REF for player
  (set `self.Character Movement` (`Character.CharacterMovement` _returnvalue))
  (set `self.Mesh` (`Character.Mesh` _returnvalue)))

(event `EnhancedInput|/Game/Player/Input/Actions/IA_Transform`
  (params (ActionValue :type Boolean) (ElapsedSeconds :type "Float (double-precision)") (TriggeredSeconds :type "Float (double-precision)") (InputAction :type "InputAction Object Reference" :default "/Game/Player/Input/Actions/IA_Transform.IA_Transform"))
  (bind _character_movement (`self.Character Movement`))
  (:`Triggered`
    (`self.IsBat?`
      (:`then`
        (`self.Transform_Human` :!label _label)
        (set `CharacterMovementComponent.GravityScale` 1.75 _character_movement)
        (set `CharacterMovementComponent.AirControl` 0.8 _character_movement)
        (set `self.IsBat?` false))
      (:`else`
        (`self.Transform_Bat`)
        (`self.SetBatGravity`)
        (set `self.IsBat?` true)))
    (`CharacterMovementComponent.SetMovementMode` (`self.Character Movement`) "MOVE_Falling" 0)
    (`self.Poof_Activated`)))

(event `ForceHumanTransform`
  (goto _label))

(fn `SetBatGravity`
  (bind _character_movement (`self.Character Movement`))
  (bind _character_movement_2 (`self.Character Movement`))
  (bind (_velocity_x _velocity_y _velocity_z) (`KismetMathLibrary.BreakVector` (`MovementComponent.Velocity` (`self.Character Movement`))))
  (bind (_velocity_x_2 _velocity_y_2 _velocity_z_2) (`KismetMathLibrary.BreakVector` (`MovementComponent.Velocity` (`self.Character Movement`))))
  ;[0.1221 0.07819 0.4179 0.502] When in Bat mode set the GRAVITY, AIR CONTROL, and VELOCITY based on wheter player is falling (and moving while falling or not)
  (if (`NavMovementComponent.IsFalling` (`self.Character Movement`))
    ;; Set Gravity and Air control
    (set `CharacterMovementComponent.GravityScale` 2.0 _character_movement)
    (set `CharacterMovementComponent.AirControl` 1.0 _character_movement)
    ;; Check to see if the player is moving
    (if (>= (`KismetMathLibrary.VSize` (`MovementComponent.Velocity` (`self.Character Movement`))) 0.001)
      ;; Clamp the max and min velocity based on if moving or not (When bat standing still dive down, when bat falling but moving glide
      (set `MovementComponent.Velocity` (`KismetMathLibrary.MakeVector` _velocity_x_2 _velocity_y_2 (`KismetMathLibrary.FClamp` _velocity_z_2 -100.0 100.0)) (`self.Character Movement`))
      (else
        (set `MovementComponent.Velocity` (`KismetMathLibrary.MakeVector` _velocity_x _velocity_y (`KismetMathLibrary.FClamp` _velocity_z -600.0 600.0)) (`self.Character Movement`))))
    (else
      (set `CharacterMovementComponent.GravityScale` 5.0 _character_movement_2)
      (set `CharacterMovementComponent.AirControl` 1.0 _character_movement_2))))

(fn `Transform_Bat`
  ;[0.1217 0.07782 0.4174 0.5] When Transform to Bat change skeletal mesh of player
  (`SkeletalMeshComponent.SetSkeletalMeshAsset` (`self.Mesh`) "/Engine/EngineMeshes/SkeletalCube.SkeletalCube")
  (set `self.IsBat?` true))

(fn `Transform_Human`
  (bind _mesh (`self.Mesh`))
  ;[0.1217 0.07782 0.4174 0.5] When transform to human, change skeletal mesh back
  (`SceneComponent.SetVisibility` _mesh true false)
  (`self.SetActive` _mesh true false))